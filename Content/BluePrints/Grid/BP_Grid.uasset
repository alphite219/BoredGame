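; BP_Grid is a tile grid actor that draws its lines and a selected-tile highlight as procedural meshes.
; The construction script builds both meshes from CreateLine quads, the highlight being one tile-thick line, with dynamic M_Grid materials for colour and opacity.
; Helpers convert between world locations and bounds-checked row/column indices relative to actor location, ignoring rotation.
; SetSelectedTile moves or hides the highlight; TileValidRadius is a stub returning false.
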(fn ConstructionScript
  (bind _tilesize (Variables|Constants|GetTileSize))
  (bind _returnvalue (/ _tilesize 2.0))
  (bind _materialinstance (Private|CreateMaterialInstance (Variables|Constants|GetLineColour) (Variables|Constants|GetLineOpacity)))
  (LocalVariables|SetLineMaterialInstance _materialinstance)
  (bind _materialinstance_2 (Private|CreateMaterialInstance (Variables|Constants|GetSelectionColour) (Variables|Constants|GetSelectionOpacity)))
  (LocalVariables|SetSelectionMaterialInstance _materialinstance_2)
  (Utilities|FlowControl|Sequence
    (:then_0
      ;[1 1 1] Create Horizontal Lines Geometry
      (for _index (range 0 (Variables|Constants|GetNumRows))
        (LocalVariables|SetLineStart (* _index (Variables|Constants|GetTileSize)))
        (bind _output_get (LocalVariables|SetLineEnd (Private|GridWidth)))
        (Private|CreateLine (Math|Vector|MakeVector (LocalVariables|GetLineStart) 0.0 0.0) (Math|Vector|MakeVector (LocalVariables|GetLineStart) _output_get 0.0) (Variables|Constants|GetLineThickness) (LocalVariables|GetLineVertices) (LocalVariables|GetLineTriangles))))
    (:then_1
      ;[1 1 1] Create Vertical Lines Geometry
      (for _index_2 (range 0 (Variables|Constants|GetNumColumns))
        (LocalVariables|SetLineStart (* _index_2 (Variables|Constants|GetTileSize)))
        (bind _output_get_2 (LocalVariables|SetLineEnd (Private|GridHeight)))
        (Private|CreateLine (Math|Vector|MakeVector 0.0 (LocalVariables|GetLineStart) 0.0) (Math|Vector|MakeVector _output_get_2 (LocalVariables|GetLineStart) 0.0) (Variables|Constants|GetLineThickness) (LocalVariables|GetLineVertices) (LocalVariables|GetLineTriangles))))
    (:then_2
      ;[1 1 1] Create Procedural Lines
      (Class|ProceduralMeshComponent|CreateMeshSectionLinearColor (Variables|Default|GetGridMesh) 0 (LocalVariables|GetLineVertices) (LocalVariables|GetLineTriangles) 0 0 0 0 0 0 0 false)
      (Rendering|Material|SetMaterial (Variables|Default|GetGridMesh) 0 (LocalVariables|GetLineMaterialInstance)))
    (:then_3
      ;[1 1 1] Create Selection Geometry
      (Private|CreateLine (Math|Vector|MakeVector 0.0 _returnvalue 0.0) (Math|Vector|MakeVector _tilesize _returnvalue 0.0) (Variables|Constants|GetTileSize) (LocalVariables|GetSelection%20Verticles) (LocalVariables|GetSelectionTriangles))
      (Rendering|SetVisibility (Variables|Default|GetSelectionMesh) false false)
      (Class|ProceduralMeshComponent|CreateMeshSectionLinearColor (Variables|Default|GetSelectionMesh) 0 (LocalVariables|GetSelection%20Verticles) (LocalVariables|GetSelectionTriangles) 0 0 0 0 0 0 0 false)
      (Rendering|Material|SetMaterial (Variables|Default|GetSelectionMesh) 0 (LocalVariables|GetSelectionMaterialInstance)))))

(fn CreateLine
  (params (Start :type Vector) (End :type Vector) (Thickness :type Float%20%28single-precision%29) (Verticies :type Array%20of%20Vectors) (Triangles :type Array%20of%20Integers))
  (bind _returnvalue (Utilities|Array|Length Verticies))
  (Utilities|FlowControl|Sequence
    (:then_0
      (LocalVariables|SetHalfThickness (/ Thickness 2.0))
      (LocalVariables|SetThicknessDirection (Math|Vector|CrossProduct (Math|Vector|Normalize (- End Start)) "0, 0,1.000000")))
    (:then_1
      (Utilities|Array|AppendArray Triangles (Utilities|Array|MakeArray (+ _returnvalue 2) (+ _returnvalue 1) (+ _returnvalue 0) (+ _returnvalue 2) (+ _returnvalue 3) (+ _returnvalue 1)))
      (Utilities|Array|AppendArray Verticies (Utilities|Array|MakeArray (+ Start (* (LocalVariables|GetThicknessDirection) (LocalVariables|GetHalfThickness))) (+ End (* (LocalVariables|GetThicknessDirection) (LocalVariables|GetHalfThickness))) (- Start (* (LocalVariables|GetThicknessDirection) (LocalVariables|GetHalfThickness))) (- End (* (LocalVariables|GetThicknessDirection) (LocalVariables|GetHalfThickness))))))))

(fn GridWidth
  (return (* (Variables|Constants|GetNumColumns) (Variables|Constants|GetTileSize))))

(fn GridHeight
  (return (* (Variables|Constants|GetNumRows) (Variables|Constants|GetTileSize))))

(fn CreateMaterialInstance
  (params (Colour :type Linear%20Color%20Structure) (Opacity :type Float%20%28single-precision%29))
  (bind _returnvalue (Rendering|Material|CreateDynamicMaterialInstance "/Game/BluePrints/Grid/M_Grid.M_Grid" "None" "None" :!class /Script/Engine.KismetMaterialLibrary))
  (Rendering|Material|SetVectorParameterValue _returnvalue "Colour" Colour :!class /Script/Engine.MaterialInstanceDynamic)
  (Rendering|Material|SetScalarParameterValue _returnvalue "Opacity" Opacity :!class /Script/Engine.MaterialInstanceDynamic)
  (return _returnvalue))

(fn LocationtoTile
  (params (Location :type Vector))
  (bind _returnvalue (Transformation|GetActorLocation))
  (bind _gridwidth (Private|GridWidth))
  (bind _gridheight (Private|GridHeight))
  (bind _returnvalue_2 (Transformation|GetActorLocation))
  (bind _numrows (Variables|Constants|GetNumRows))
  (bind _numcolumns (Variables|Constants|GetNumColumns))
  (bind _returnvalue_3 (- (.y Location) (.y _returnvalue)))
  (bind _returnvalue_4 (- (.x Location) (.x _returnvalue_2)))
  (bind _returnvalue_5 (/ _returnvalue_4 _gridheight))
  (bind _returnvalue_6 (/ _returnvalue_3 _gridwidth))
  (bind _returnvalue_7 (* _numrows _returnvalue_5))
  (bind _returnvalue_8 (* _numcolumns _returnvalue_6))
  (bind _returnvalue_9 (Math|Float|Floor _returnvalue_7))
  (bind _returnvalue_10 (Math|Float|Floor _returnvalue_8))
  (bind _valid (Utilities|TileValid _returnvalue_9 _returnvalue_10))
  (return _valid _returnvalue_9 _returnvalue_10))

(fn TiletoGridLocation
  (params (Row :type Integer) (Column :type Integer) (Center? :type Boolean))
  (bind _returnvalue (Transformation|GetActorLocation))
  (bind _tilesize (Variables|Constants|GetTileSize))
  (bind _returnvalue_2 (/ _tilesize 2.0))
  (bind _returnvalue_3 (select Center? _returnvalue_2 0.0))
  (bind _valid (Utilities|TileValid Row Column))
  (return _valid (Math|Vector2D|MakeVector2D (+ (+ (* Row (Variables|Constants|GetTileSize)) (.x _returnvalue)) _returnvalue_3) (+ (+ (.y _returnvalue) (* Column (Variables|Constants|GetTileSize))) _returnvalue_3))))

(fn SetSelectedTile
  (params (Row :type Integer) (Colomn :type Integer))
  (bind _selectionmesh (Variables|Default|GetSelectionMesh))
  (bind (_valid_ _gridlocation) (CallFunction|TiletoGridLocation Row Colomn false))
  (if _valid_
    (Rendering|SetVisibility _selectionmesh true false)
    (Transformation|SetWorldLocation (Variables|Default|GetSelectionMesh) (Math|Vector|MakeVector (.X (Math|Vector2D|BreakVector2D _gridlocation)) (.Y (Math|Vector2D|BreakVector2D _gridlocation)) (.z (Transformation|GetActorLocation))) false false)
    (else
      (Rendering|SetVisibility _selectionmesh false false))))

(fn TileValidRadius
  (params (Row :type Integer) (Column :type Integer))
  (return false))

(fn LocationtoTileChecking
  (params (Location :type Vector) (CompareRow :type Integer) (CompareColomn :type Integer))
  (bind _returnvalue (Transformation|GetActorLocation))
  (bind _gridwidth (Private|GridWidth))
  (bind _gridheight (Private|GridHeight))
  (bind _returnvalue_2 (Transformation|GetActorLocation))
  (bind _numrows (Variables|Constants|GetNumRows))
  (bind _numcolumns (Variables|Constants|GetNumColumns))
  (bind _returnvalue_3 (- (.y Location) (.y _returnvalue)))
  (bind _returnvalue_4 (- (.x Location) (.x _returnvalue_2)))
  (bind _returnvalue_5 (/ _returnvalue_4 _gridheight))
  (bind _returnvalue_6 (/ _returnvalue_3 _gridwidth))
  (bind _returnvalue_7 (* _numrows _returnvalue_5))
  (bind _returnvalue_8 (* _numcolumns _returnvalue_6))
  (bind _returnvalue_9 (Math|Float|Floor _returnvalue_7))
  (bind _returnvalue_10 (Math|Float|Floor _returnvalue_8))
  (bind _valid (Utilities|TileValid _returnvalue_9 _returnvalue_10))
  (return _valid _returnvalue_9 _returnvalue_10))