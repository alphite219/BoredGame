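; GM_Default is a game mode Blueprint that holds a grid reference and early dice-roll logic.
; BeginPlay caches the first BP_Grid actor for GetGrid, printing a warning if none exists.
; CallDiceRoll sends ApplyDamageMessage to the player character with a Select fixed at index zero, so damage is always 1.
; RollDice only prints a random side from DiceTpye, and TurnSystem is an empty stub.
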(event Custom|CallDiceRoll
  (bind _returnvalue (Utilities|Select :Index 0 :Option%200 1 :Option%201 2 :Option%202 3 :Option%203 4 :Option%204 5 :Option%205 6))
  (Development|PrintString (Utilities|String|ToString(Integer) _returnvalue))
  (Class|BPIDamage|ApplyDamage(Message) (Game|GetPlayerCharacter 0) _returnvalue))

(event Custom|TurnSystem)

(event EventBeginPlay
  (bind _outactors (Actor|GetAllActorsOfClass "/Game/BluePrints/Grid/BP_Grid.BP_Grid_C"))
  (Utilities|IsValid (Utilities|Array|Get(acopy) _outactors)
    (:Is%20Valid
      (Variables|Private|SetGrid (Utilities|Array|Get(acopy) _outactors)))
    (:Is%20Not%20Valid
      (Development|PrintString "No Grid"))))

(fn ConstructionScript)

(fn GetGrid
  (return (Variables|Private|GetGrid)))

(fn RollDice
  (Development|PrintString (Utilities|String|ToString(Integer) (.OutItem (Utilities|Array|Random (Variables|/Game/BluePrints/Dice/DAP_DiceTypes.DAP_DiceTypes_C|GetSides (Variables|Default|GetDiceTpye)))))))