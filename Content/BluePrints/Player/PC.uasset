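; Player controller for click-to-move on a tile grid, limited by the player pawn's remaining movement count.
; While SetDestination is held, Tick traces under the cursor through a gate and a DoOnce that resets after each attempt, with a short delay after a move.
; Each attempt spends a move, then uses the game mode's grid to allow only orthogonally adjacent tiles, pathing to the tile center.
; Non-adjacent targets refund the spent move.
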(event Custom|ResetGate
  (bind _playerbp (Variables|Default|GetPlayerBP))
  (Utilities|FlowControl|DoOnce false) ; enters at Reset
)

(event EventBeginPlay
  (bind _asbp_player (Utilities|Casting|CastToBP_Player (Game|GetPlayerCharacter 0)))
  (Variables|Default|SetPlayerBP _asbp_player))

(event EventTick
  (params (DeltaSeconds :type Float%20%28single-precision%29))
  (bind (_hitresult _returnvalue) (Game|Player|GetHitResultUnderCursorbyChannel "TraceTypeQuery1" true))
  (bind _playerbp (Variables|Default|GetPlayerBP))
  (Utilities|FlowControl|Sequence
    (:then_0
      (Utilities|FlowControl|Gate true ; While key is pressed...
        (:Exit
          (if _returnvalue
            (Utilities|FlowControl|DoOnce false
              (:Completed
                (if (> (Variables|/Game/BluePrints/Player/BP_Player.BP_Player_C|GetMovementNumber (Variables|Default|GetPlayerBP)) 0)
                  (Variables|/Game/BluePrints/Player/BP_Player.BP_Player_C|SetMovementNumber _playerbp (- (Variables|/Game/BluePrints/Player/BP_Player.BP_Player_C|GetMovementNumber _playerbp) 1))
                  (CallFunction|MovetoHitLocation _hitresult) ; ..and move there.
                  (Utilities|FlowControl|Delay 0.5)
                  (CallFunction|ResetGate)
                  (else
                    (CallFunction|ResetGate)))))))))))

(event Input|ActionEvents|InputActionSetDestination
  (params (Key :type Key%20Structure :default "None"))
  (bind (_hitresult _returnvalue) (Game|Player|GetHitResultUnderCursorbyChannel "TraceTypeQuery1" true))
  (bind _playerbp (Variables|Default|GetPlayerBP))
  (:Pressed
    (Utilities|FlowControl|Gate true) ; enters at Open
  )
  (:Released
    (Utilities|FlowControl|Gate true) ; enters at Close
  ))

(fn ConstructionScript)

(fn MovetoHitLocation
  (params (Hit :type Hit%20Result%20Structure))
  (bind _location (Collision|BreakHitResult Hit))
  (bind _playerbp (Variables|Default|GetPlayerBP))
  (if (>= (Math|Vector|VectorLength (- (Transformation|GetActorLocation (Pawn|GetControlledPawn)) _location)) (Variables|Default|GetMinClickDistance)) ; Don't move if player clicks too close to pawn
    (LocalVariables|SetHitLocation _location)
    (bind _asgm_default (Utilities|Casting|CastToGM_Default (Game|GetGameMode)))
    (bind (_valid _row _column) (Default|LocationtoTile (Default|GetGrid _asgm_default) (LocalVariables|GetHitLocation)))
    (bind (_valid_2 _row_2 _column_2) (Default|LocationtoTile (Default|GetGrid _asgm_default) (Transformation|GetActorLocation (Variables|Default|GetPlayerBP))))
    (if (or (and (== _row _row_2) (or (== _column (+ _column_2 1)) (== _column (- _column_2 1)))) (and (== _column_2 _column) (or (== _row (+ _row_2 1)) (== _row (- _row_2 1)))))
      (bind _gridlocation (Default|TiletoGridLocation (Default|GetGrid _asgm_default) _row _column true))
      (AI|Navigation|SimpleMovetoLocation self (Math|Vector|MakeVector (.x _gridlocation) (.y _gridlocation) (.z (LocalVariables|GetHitLocation))))
      (else
        (Variables|/Game/BluePrints/Player/BP_Player.BP_Player_C|SetMovementNumber _playerbp (+ (Variables|/Game/BluePrints/Player/BP_Player.BP_Player_C|GetMovementNumber _playerbp) 1))))))