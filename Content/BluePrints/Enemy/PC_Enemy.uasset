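; Enemy controller that moves its BP_Enemy pawn around the game mode's grid in random steps and triggers attacks.
; MoveAmount repeats MoveToLocation on a delay, picking a 200-unit axis offset (two of four cases both use -Y) and snapping it to a tile center.
; It attacks instead if that target tile is orthogonally adjacent to the cached player tile, which only refreshes through GetPlayerPosition, called by CheckCurrentPosition.
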(event Custom|MoveAmount
  (params (MoveAmount :type Integer))
  (Utilities|ForEachwithBreakDelay 0 MoveAmount 1.0
    (:Loop%20Body
      (Development|PrintString "Move")
      (CallFunction|MovetoLocation))))

(event EventBeginPlay
  (bind _asgm_default (Utilities|Casting|CastToGM_Default (Game|GetGameMode)))
  (Variables|Default|SetGrid (Default|GetGrid _asgm_default))
  (bind _asbp_enemy (Utilities|Casting|CastToBP_Enemy (Pawn|GetControlledPawn)))
  (Variables|Default|SetEnemyRef _asbp_enemy))

(fn ConstructionScript)

(fn MovetoLocation
  (bind _output_get (LocalVariables|SetCurrentLocation (Transformation|GetActorLocation (Variables|Default|GetEnemyRef))))
  (switch int (Math|Random|RandomIntegerinRange 0 3)
    (:0
      (LocalVariables|SetTargetLocation (Math|Vector|MakeVector (+ (.x _output_get) 2e+02) (.y _output_get) (.z _output_get))))
    (:1
      (LocalVariables|SetTargetLocation (Math|Vector|MakeVector (+ (.x (LocalVariables|GetCurrentLocation)) -2e+02) (.y (LocalVariables|GetCurrentLocation)) (.z (LocalVariables|GetCurrentLocation)))))
    (:2
      (LocalVariables|SetTargetLocation (Math|Vector|MakeVector (.x (LocalVariables|GetCurrentLocation)) (+ (.y (LocalVariables|GetCurrentLocation)) -2e+02) (.z (LocalVariables|GetCurrentLocation)))))
    (:3
      (LocalVariables|SetTargetLocation (Math|Vector|MakeVector (.x (LocalVariables|GetCurrentLocation)) (+ (.y (LocalVariables|GetCurrentLocation)) -2e+02) (.z (LocalVariables|GetCurrentLocation))))))
  (bind (_valid _row _column) (Default|LocationtoTile (Variables|Default|GetGrid) (LocalVariables|GetTargetLocation)))
  (LocalVariables|SetRow _row)
  (LocalVariables|SetColomn _column)
  (if (Math|Boolean|ORBoolean (and (== (LocalVariables|GetRow) (+ (Variables|Default|GetPlayerRow) 1)) (== (Variables|Default|GetPlayerColumn) (LocalVariables|GetColomn))) (and (== (LocalVariables|GetRow) (+ (Variables|Default|GetPlayerRow) -1)) (== (Variables|Default|GetPlayerColumn) (LocalVariables|GetColomn))) (and (== (LocalVariables|GetColomn) (+ (Variables|Default|GetPlayerColumn) 1)) (== (LocalVariables|GetRow) (Variables|Default|GetPlayerRow))) (and (== (LocalVariables|GetColomn) (+ (Variables|Default|GetPlayerColumn) -1)) (== (LocalVariables|GetRow) (Variables|Default|GetPlayerRow))))
    (Default|Attack (Variables|Default|GetEnemyRef))
    (else
      (bind _gridlocation (Default|TiletoGridLocation (Variables|Default|GetGrid) (LocalVariables|GetRow) (LocalVariables|GetColomn) true))
      (AI|Navigation|SimpleMovetoLocation self (Math|Vector|MakeVector (.x _gridlocation) (.y _gridlocation) (.z (LocalVariables|GetCurrentLocation)))))))

(fn GetPlayerPosition
  (bind (_valid _row _column) (Default|LocationtoTile (Variables|Default|GetGrid) (Transformation|GetActorLocation (Game|GetPlayerCharacter 0))))
  (Variables|Default|SetPlayerRow _row)
  (Variables|Default|SetPlayerColumn _column))

(fn CheckCurrentPosition
  (CallFunction|GetPlayerPosition)
  (bind (_valid _row _column) (Default|LocationtoTile (Variables|Default|GetGrid) (Transformation|GetActorLocation)))
  (LocalVariables|SetRow _row)
  (LocalVariables|SetColumn _column)
  (return (Math|Boolean|ORBoolean (and (== (LocalVariables|GetRow) (+ (Variables|Default|GetPlayerRow) 1)) (== (Variables|Default|GetPlayerColumn) (LocalVariables|GetColumn))) (and (== (LocalVariables|GetRow) (+ (Variables|Default|GetPlayerRow) -1)) (== (Variables|Default|GetPlayerColumn) (LocalVariables|GetColumn))) (and (== (LocalVariables|GetColumn) (+ (Variables|Default|GetPlayerColumn) 1)) (== (LocalVariables|GetRow) (Variables|Default|GetPlayerRow))) (and (== (LocalVariables|GetColumn) (+ (Variables|Default|GetPlayerColumn) -1)) (== (LocalVariables|GetRow) (Variables|Default|GetPlayerRow))))))